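; Debug variant of the HuMa character that binds keyboard keys to test abilities and interaction.
; P and X activate the auto-attack and Warrior main abilities through the Ability System Component, while E begins and ends interaction.
; O calls a server test on every other press with the main target and ASC.
; A Server_test event applies the weapons-out gameplay effect, gated by FlipFlop and DoOnce.
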(event `Key|P`
  (params (Key :type "Key Structure"))
  (:`Pressed`
    (`AbilitySystemComponent.TryActivateAbilityByClass` (`AbilitySystemBlueprintLibrary.GetAbilitySystemComponent` self) "/Game/XIRemix/Abilities/GA_AutoAttack.GA_AutoAttack_C" true)))

(event `Key|X`
  (params (Key :type "Key Structure"))
  (:`Pressed`
    (`AbilitySystemComponent.TryActivateAbilityByClass` (`AbilitySystemBlueprintLibrary.GetAbilitySystemComponent` self) "/Game/XIRemix/Abilities/Jobs/GA_Warrior_Main.GA_Warrior_Main_C" true)))

(event `Key|E`
  (params (Key :type "Key Structure"))
  (:`Pressed`
    (`self.BeginInteract`))
  (:`Released`
    (`self.EndInteract`)))

(event `Key|O`
  (params (Key :type "Key Structure"))
  (:`Pressed`
    (`/Engine/EditorBlueprintResources/StandardMacros.FlipFlop`
      (:`A`
        (`self.Server_test` (`self.MainTarget`) (`AbilitySystemBlueprintLibrary.GetAbilitySystemComponent` self))))))

(event `Server_test`
  (params (Actor :type "Actor Object Reference") (ASC :type "AbilitySystemComponent Object Reference"))
  (`/Engine/EditorBlueprintResources/StandardMacros.FlipFlop`
    (:`A`
      (`/Engine/EditorBlueprintResources/StandardMacros.DoOnce` false
        (:`Completed`
          (`AbilitySystemComponent.BP_ApplyGameplayEffectToSelf` :`self` ASC :`GameplayEffectClass` "/Game/XIRemix/Abilities/_Test/GE_SetWeaponsOut.GE_SetWeaponsOut_C"))))))

(fn `UserConstructionScript`)