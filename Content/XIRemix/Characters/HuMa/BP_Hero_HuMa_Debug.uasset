(event `self.ReceiveBeginPlay`
  (bind _returnvalue (`MeshMergeFunctionLibrary.MergeMeshes` (`self.SK_MeshMergeParams`)))
  (`/Engine/EditorBlueprintResources/StandardMacros.IsValid` _returnvalue
    (:`Is Valid`
      (`SkinnedMeshComponent.SetSkinnedAssetAndUpdate` (`self.Mesh`) _returnvalue false))))

(event `Key|I`
  (params (Key :type "Key Structure"))
  ;[1 1 1] Combat Montage Testing
  (:`Pressed`
    (`self.Server_PlayAnimMontage` (`self.GetAutoAttackMontage_CPP`))))

(event `Key|O`
  (params (Key :type "Key Structure"))
  ;[1 1 1] Combat Montage Testing
  (:`Pressed`
    (`self.Server_DebugEvent_StartCombat`)))

(event `Key|P`
  (params (Key :type "Key Structure"))
  (:`Pressed`
    (`AbilitySystemComponent.TryActivateAbilityByClass` (`AbilitySystemBlueprintLibrary.GetAbilitySystemComponent` self) "/Game/XIRemix/Abilities/GA_TestAttack.GA_TestAttack_C" true)))

(event `Server_DebugEvent_StartCombat`
  (bind _returnvalue (`AbilitySystemBlueprintLibrary.GetAbilitySystemComponent` self))
  ;[1 1 1] Combat Montage Testing
  (bind _isa (`/Engine/EditorBlueprintResources/StandardMacros.FlipFlop`)
    (:`A`
      _)
    (:`B`
      _))
  (`self.Multi_DebugEvent_StartCombat` _isa)
  (`KismetSystemLibrary.Delay` (`AnimSequenceBase.SequenceLength` (`self.GetCombatStartMontage`)))
  (if _isa
    (`AbilitySystemComponent.BP_ApplyGameplayEffectToSelf` :`self` _returnvalue :`GameplayEffectClass` "/Game/XIRemix/Abilities/GE_SetWeaponsOut.GE_SetWeaponsOut_C" :`Level` 1.0)
    (else
      (`AbilitySystemComponent.RemoveActiveEffectsWithGrantedTags` _returnvalue (struct :`GameplayTags` (struct :`(TagName` "State.Gameplay.WeaponsOut")))))))

(event `Multi_DebugEvent_StartCombat`
  (params (Condition :type Boolean))
  ;[1 1 1] Combat Montage Testing
  (if Condition
    (`self.PlayAnimMontage` (`self.GetCombatStartMontage`))
    (else
      (`self.PlayAnimMontage` (`self.GetCombatExitMontage`))))
  (message `AnimBPInterface.SetCombatStyle` (`SkeletalMeshComponent.GetAnimInstance` (`self.Mesh`)) (`self.CombatStyle`)))

(fn `UserConstructionScript`
  (`parent.UserConstructionScript`))