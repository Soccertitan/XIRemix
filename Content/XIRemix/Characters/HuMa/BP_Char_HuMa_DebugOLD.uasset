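; Debug character Blueprint for HuMa, marked old by its name, that triggers Gameplay Ability System abilities from hardcoded keys.
; X and P directly activate the Warrior main and auto-attack abilities on the character's ability system component.
; O calls a server test on alternate presses, passing that component and the main target.
; The Server_test event activates the Warrior ability behind FlipFlop and DoOnce gates, ignoring its actor input.
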(event `Key|X`
  (params (Key :type "Key Structure"))
  (:`Pressed`
    (`AbilitySystemComponent.TryActivateAbilityByClass` (`AbilitySystemBlueprintLibrary.GetAbilitySystemComponent` self) "/Game/XIRemix/Abilities/Jobs/GA_Warrior_Main.GA_Warrior_Main_C" true)))

(event `Key|P`
  (params (Key :type "Key Structure"))
  (:`Pressed`
    (`AbilitySystemComponent.TryActivateAbilityByClass` (`AbilitySystemBlueprintLibrary.GetAbilitySystemComponent` self) "/Game/XIRemix/Abilities/GA_AutoAttack.GA_AutoAttack_C" true)))

(event `Key|One`
  (params (Key :type "Key Structure")))

(event `Key|O`
  (params (Key :type "Key Structure"))
  (:`Pressed`
    (`/Engine/EditorBlueprintResources/StandardMacros.FlipFlop`
      (:`A`
        (`self.Server_test` (`AbilitySystemBlueprintLibrary.GetAbilitySystemComponent` self) (`self.MainTarget`))))))

(event `Server_test`
  (params (Target :type "AbilitySystemComponent Object Reference") (Actor :type "Actor Object Reference"))
  (`/Engine/EditorBlueprintResources/StandardMacros.FlipFlop`
    (:`A`
      (`/Engine/EditorBlueprintResources/StandardMacros.DoOnce` false
        (:`Completed`
          (`AbilitySystemComponent.TryActivateAbilityByClass` Target "/Game/XIRemix/Abilities/Jobs/GA_Warrior_Main.GA_Warrior_Main_C" true))))))

(fn `UserConstructionScript`)