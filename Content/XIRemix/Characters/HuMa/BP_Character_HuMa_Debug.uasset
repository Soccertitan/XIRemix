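; Debug variant of the HuMa character for exercising mesh merging and the Gameplay Ability System.
; On BeginPlay it merges skeletal meshes from merge params and, if the result is valid, applies it to the character mesh.
; Debug keys activate the auto-attack ability (P) and call a server test event that applies a buff effect to the ability system component (O).
; An attribute-override test effect is left unconnected.
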(event `self.ReceiveBeginPlay`
  (bind _returnvalue (`MeshMergeFunctionLibrary.MergeMeshes` (`self.SKMeshMergeParams`)))
  (`/Engine/EditorBlueprintResources/StandardMacros.IsValid` _returnvalue
    (:`Is Valid`
      (`SkinnedMeshComponent.SetSkinnedAssetAndUpdate` (`self.Mesh`) _returnvalue false))))

(event `Key|P`
  (params (Key :type "Key Structure"))
  (:`Pressed`
    (`AbilitySystemComponent.TryActivateAbilityByClass` (`AbilitySystemBlueprintLibrary.GetAbilitySystemComponent` self) "/Game/XIRemix/Abilities/Common/GA_AutoAttack.GA_AutoAttack_C" true)))

(event `Key|O`
  (params (Key :type "Key Structure"))
  (:`Pressed`
    (`self.Server_test` (`AbilitySystemBlueprintLibrary.GetAbilitySystemComponent` self))))

(event `Server_test`
  (params (Target :type "AbilitySystemComponent Object Reference"))
  (`AbilitySystemComponent.BP_ApplyGameplayEffectToSelf` :`self` Target :`GameplayEffectClass` "/Game/XIRemix/Abilities/GE_SetBuff.GE_SetBuff_C"))

(fn `UserConstructionScript`)