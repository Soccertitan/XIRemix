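; Player hero base character Blueprint that handles switching the current target among nearby actors.
; The IA_TargetRight input passes its action value as a direction to TargetActor, along with the XITargetSystem component and SphereTargetCollision.
; TargetActor rebuilds PerceivedActors from overlapping actors whose Ability System Component matches a gameplay tag filter, which the input event leaves unset.
; It then hands that list and direction to the target system's SwitchTargetActor.
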(event `EnhancedInput|/Game/XIRemix/Core/Player/Input/IA_TargetRight`
  (params (ActionValue :type "Float (single-precision)") (ElapsedSeconds :type "Float (single-precision)") (TriggeredSeconds :type "Float (single-precision)"))
  (:`Triggered`
    (`self.TargetActor` (`self.XITargetSystem`) (struct :`TagName` "Faction.Enemy") (`self.SphereTargetCollision`) ActionValue)))

(fn `TargetActor`
  (params (TargetSystemComponent :type "XITargetSystemComponent Object Reference") (GameplayTagFilter :type "GameplayTag Structure" :default (struct :`TagName` "Faction.Enemy")) (TargetCollision :type "PrimitiveComponent Object Reference") (Direction :type "Float (double-precision)"))
  (`KismetArrayLibrary.Array_Clear` (`self.PerceivedActors`))
  (for _array_element (`PrimitiveComponent.GetOverlappingActors` TargetCollision null)
    (bind _returnvalue (`AbilitySystemBlueprintLibrary.GetAbilitySystemComponent` _array_element))
    (`/Engine/EditorBlueprintResources/StandardMacros.IsValid` _returnvalue
      (:`Is Valid`
        (if (`GameplayTagAssetInterface.HasMatchingGameplayTag` _returnvalue GameplayTagFilter)
          (`KismetArrayLibrary.Array_Add` (`self.PerceivedActors`) _array_element)))))
  (`XITargetSystemComponent.SwitchTargetActor` TargetSystemComponent (`self.PerceivedActors`) Direction))

(fn `UserConstructionScript`)