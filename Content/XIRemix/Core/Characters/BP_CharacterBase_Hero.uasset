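; Base hero character Blueprint that handles player targeting, camera lock-on and the target plate UI.
; Target-switch input gathers tag-filtered actors with ability system components from XITargetSphere overlaps, then passes them and the input direction to XITargetSystem.
; Target system selection and removal events create and remove the WBP_TargetPlate widget.
; A Q debug key sends the target's ability system component to a server event that applies a test damage GameplayEffect.
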(event `EnhancedInput|/Game/XIRemix/Core/Player/Input/IA_TargetRight`
  (params (ActionValue :type "Float (single-precision)") (ElapsedSeconds :type "Float (single-precision)") (TriggeredSeconds :type "Float (single-precision)"))
  (:`Triggered`
    (`self.TargetActor` (`self.XITargetSystem`) (struct :`TagName` "Faction.Enemy") (`self.XITargetSphere`) ActionValue)))

(event `EnhancedInput|/Game/XIRemix/Core/Player/Input/IA_TargetLock`
  (params (ActionValue :type Boolean) (ElapsedSeconds :type "Float (single-precision)") (TriggeredSeconds :type "Float (single-precision)"))
  (:`Triggered`
    (`XITargetSystemComponent.LockCamera` (`self.XITargetSystem`))))

(event `self.XITargetSystem.OnTargetSelected`
  (params (TargetActor :type "Actor Object Reference"))
  (`self.TargetUI`
    (:`then`)
    (:`else`
      (bind _returnvalue (`|CreateWidget` "/Game/XIRemix/Core/Player/UI/WBP_TargetPlate.WBP_TargetPlate_C" (`GameplayStatics.GetPlayerController` 0) TargetActor))
      (bind _output_get (set `self.TargetUI` _returnvalue))
      (`UserWidget.AddToViewport` _output_get 0))))

(event `self.XITargetSystem.OnTargetRemoved`
  (params (TargetActor :type "Actor Object Reference"))
  (bind _targetui (`self.TargetUI`)
    (:`then`
      (`Widget.RemoveFromParent` _targetui)
      (set `self.TargetUI` null))
    (:`else`)))

(event `Key|Q`
  (params (Key :type "Key Structure"))
  (bind _returnvalue (`AbilitySystemBlueprintLibrary.GetAbilitySystemComponent` (`XITargetSystemComponent.GetTargetedActor` (`self.XITargetSystem`))))
  (:`Pressed`
    (`/Engine/EditorBlueprintResources/StandardMacros.IsValid` _returnvalue
      (:`Is Valid`
        (`self.Server_ApplyGE` _returnvalue)))))

(event `Server_ApplyGE`
  (params (Target :type "AbilitySystemComponent Object Reference"))
  (`AbilitySystemComponent.BP_ApplyGameplayEffectToSelf` :`self` Target :`GameplayEffectClass` "/Game/XIRemix/Abilities/GE_TestDamage.GE_TestDamage_C"))

(fn `TargetActor`
  (params (TargetSystemComponent :type "XITargetSystemComponent Object Reference") (GameplayTagFilter :type "GameplayTag Structure" :default (struct :`TagName` "Faction.Enemy")) (TargetCollision :type "PrimitiveComponent Object Reference") (Direction :type "Float (double-precision)"))
  (`KismetArrayLibrary.Array_Clear` (`self.PerceivedActors`))
  (for _array_element (`PrimitiveComponent.GetOverlappingActors` TargetCollision null)
    (bind _returnvalue (`AbilitySystemBlueprintLibrary.GetAbilitySystemComponent` _array_element))
    (`/Engine/EditorBlueprintResources/StandardMacros.IsValid` _returnvalue
      (:`Is Valid`
        (if (`GameplayTagAssetInterface.HasMatchingGameplayTag` _returnvalue GameplayTagFilter)
          (`KismetArrayLibrary.Array_Add` (`self.PerceivedActors`) _array_element)))))
  (`XITargetSystemComponent.SwitchTargetActor` TargetSystemComponent (`self.PerceivedActors`) Direction))

(fn `UserConstructionScript`)