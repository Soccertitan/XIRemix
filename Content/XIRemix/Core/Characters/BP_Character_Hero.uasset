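; Player hero character Blueprint that handles target selection and modular skeletal mesh appearance.
; Input actions drive XITargetSystem to pick hostile targets directionally or lock the camera.
; Target system events create or remove the target plate widget and track MainTarget.
; A server event swaps the mesh for a given part type in the merge parameters, then a multi event merges the parts and applies the result to the character mesh.
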(event `Server_MeshMerge`
  (params (SkeletalMeshType :type "ESkeletalMeshMergeType Enum (by ref)") (SkeletalMesh :type "SkeletalMesh Object Reference (by ref)"))
  (`KismetArrayLibrary.Array_Set` (`.MeshesToMerge` (break `SkeletalMeshMergeParams` (`self.SKMeshMergeParams`))) (`BlueprintMapLibrary.Map_Find` (`self.SKMeshMergeMap`) SkeletalMeshType) SkeletalMesh)
  (`self.Multi_MeshMerge`))

(event `Multi_MeshMerge`
  (bind _returnvalue (`MeshMergeFunctionLibrary.MergeMeshes` (`self.SKMeshMergeParams`)))
  (`/Engine/EditorBlueprintResources/StandardMacros.IsValid` _returnvalue
    (:`Is Valid`
      (`SkinnedMeshComponent.SetSkinnedAssetAndUpdate` (`self.Mesh`) _returnvalue false))))

(event `EnhancedInput|/Game/XIRemix/Core/Player/Input/IA_TargetRight`
  (params (ActionValue :type "Float (single-precision)") (ElapsedSeconds :type "Float (single-precision)") (TriggeredSeconds :type "Float (single-precision)"))
  (:`Triggered`
    (`XITargetSystemComponent.TargetActor` (`self.XITargetSystem`) "Hostile" ActionValue)))

(event `EnhancedInput|/Game/XIRemix/Core/Player/Input/IA_TargetLock`
  (params (ActionValue :type Boolean) (ElapsedSeconds :type "Float (single-precision)") (TriggeredSeconds :type "Float (single-precision)"))
  (:`Triggered`
    (`XITargetSystemComponent.LockCamera` (`self.XITargetSystem`))))

(event `self.XITargetSystem.OnTargetSelected`
  (params (TargetActor :type "Actor Object Reference"))
  (`self.TargetUI`
    (:`then`)
    (:`else`
      (bind _returnvalue (`|CreateWidget` "/Game/XIRemix/Core/Player/UI/WBP_TargetPlate.WBP_TargetPlate_C" (`GameplayStatics.GetPlayerController` 0) TargetActor))
      (bind _output_get (set `self.TargetUI` _returnvalue))
      (`UserWidget.AddToViewport` _output_get 0)
      (set `self.MainTarget` TargetActor))))

(event `self.XITargetSystem.OnTargetRemoved`
  (params (TargetActor :type "Actor Object Reference"))
  (bind _targetui (`self.TargetUI`)
    (:`then`
      (`Widget.RemoveFromParent` _targetui)
      (set `self.TargetUI` null)
      (set `self.MainTarget` null))
    (:`else`)))

(fn `UserConstructionScript`)