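; Debug hero character Blueprint for testing modular mesh merging and sword combat stance transitions.
; On BeginPlay it merges the SKMeshMerge mesh parts and applies the result to the character mesh.
; Pressing I calls a server event that writes a leather vest into the merge list without re-merging, then calls a multi event.
; That event alternates sword draw and sheathe montages and passes the weapons-out state to the AnimInstance.
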(event `self.ReceiveBeginPlay`
  (bind _returnvalue (`MeshMergeFunctionLibrary.MergeMeshes` (`self.SK_Mesh_Merge`)))
  (`/Engine/EditorBlueprintResources/StandardMacros.IsValid` _returnvalue
    (:`Is Valid`
      (`SkinnedMeshComponent.SetSkinnedAssetAndUpdate` (`self.Mesh`) _returnvalue true))))

(event `Key|I`
  (params (Key :type "Key Structure"))
  (:`Pressed`
    (`self.Server_DebugEvent`)))

(event `Key|O`
  (params (Key :type "Key Structure")))

(event `Server_DebugEvent`
  (`KismetArrayLibrary.Array_Set` (`.MeshesToMerge` (break `SkeletalMeshMergeParams` (`self.SK_Mesh_Merge`))) 2 "/Game/XIRemix/Characters/HuMa/Body/SK_HuMa_LeatherVest.SK_HuMa_LeatherVest")
  (`self.Multi_DebugEvent`))

(event `Multi_DebugEvent`
  (bind _isa (`/Engine/EditorBlueprintResources/StandardMacros.FlipFlop`)
    (:`A`
      (`self.PlayAnimMontage` "/Game/XIRemix/Characters/HuMa/Animations/A_Combat_Start_Sword_Montage.A_Combat_Start_Sword_Montage"))
    (:`B`
      (`self.PlayAnimMontage` "/Game/XIRemix/Characters/HuMa/Animations/A_Combat_Exit_Sword_Montage.A_Combat_Exit_Sword_Montage")))
  (message `/Game/XIRemix/Core/Interfaces/INT_AnimBP.SetCombat` (`SkeletalMeshComponent.GetAnimInstance` (`self.Mesh`)) "NewEnumerator0" _isa))

(fn `UserConstructionScript`
  (`parent.UserConstructionScript`))