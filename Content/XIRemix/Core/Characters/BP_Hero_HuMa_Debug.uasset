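; Debug hero character for testing unarmed combat animation over the network, with a body mesh built at BeginPlay by merging skeletal meshes.
; The I key requests an unarmed basic attack, and O toggles combat stance via server-to-multicast events.
; The multicast plays enter or exit montages and updates the AnimInstance's combat style and weapons-out state.
; A separate server event alternates two hand-to-hand attack montages, but nothing here calls it.
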(event `self.ReceiveBeginPlay`
  (bind _returnvalue (`MeshMergeFunctionLibrary.MergeMeshes` (`self.SK_MeshMergeParams`)))
  (`/Engine/EditorBlueprintResources/StandardMacros.IsValid` _returnvalue
    (:`Is Valid`
      (`SkinnedMeshComponent.SetSkinnedAssetAndUpdate` (`self.Mesh`) _returnvalue false))))

(event `Key|I`
  (params (Key :type "Key Structure"))
  (:`Pressed`
    (`self.Server_BasicAttack` "Unarmed")))

(event `Key|O`
  (params (Key :type "Key Structure"))
  (:`Pressed`
    (`self.Server_DebugEvent_StartCombat`)))

(event `Server_DebugEvent_StartCombat`
  (bind _isa (`/Engine/EditorBlueprintResources/StandardMacros.FlipFlop`)
    (:`A`
      _)
    (:`B`
      _))
  (`self.Multi_DebugEvent_StartCombat` _isa))

(event `Multi_DebugEvent_StartCombat`
  (params (Condition :type Boolean))
  (if Condition
    (bind _returnvalue (`self.PlayAnimMontage` "/Game/XIRemix/Characters/HuMa/Animations/AM_Combat_Start_Unarmed.AM_Combat_Start_Unarmed"))
    (`KismetSystemLibrary.Delay` _returnvalue)
    (else
      (bind _returnvalue_2 (`self.PlayAnimMontage` "/Game/XIRemix/Characters/HuMa/Animations/AM_Combat_Exit_Unarmed.AM_Combat_Exit_Unarmed"))
      (`KismetSystemLibrary.Delay` _returnvalue_2)))
  (message `/Game/XIRemix/Core/Interfaces/INT_AnimBP.SetCombat` (`SkeletalMeshComponent.GetAnimInstance` (`self.Mesh`)) (`self.CombatStyle`) Condition))

(event `Server_DebugEvent_Atk`
  (`/Engine/EditorBlueprintResources/StandardMacros.FlipFlop`
    (:`A`
      (`self.Multi_DebugEvent_Atk` "/Game/XIRemix/Characters/HuMa/Animations/AM_Atk_H2H_2.AM_Atk_H2H_2"))
    (:`B`
      (`self.Multi_DebugEvent_Atk` "/Game/XIRemix/Characters/HuMa/Animations/AM_Atk_H2H_1.AM_Atk_H2H_1"))))

(event `Multi_DebugEvent_Atk`
  (params (AnimMontage :type "AnimMontage Object Reference"))
  (`self.PlayAnimMontage` AnimMontage))

(fn `UserConstructionScript`
  (`parent.UserConstructionScript`))