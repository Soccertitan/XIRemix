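; PC_XIAction is a player controller that handles Enhanced Input for movement and camera look.
; On BeginPlay it adds the exploration and target mapping contexts at equal priority and caches the controlled pawn.
; While that pawn is valid, movement input follows the forward and right vectors of its full control rotation, and camera input drives controller pitch and yaw.
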(event `self.ReceiveBeginPlay`
  (bind _returnvalue (pcsubsystem `EnhancedInputLocalPlayerSubsystem` self))
  (message `EnhancedInputSubsystemInterface.AddMappingContext` _returnvalue "/Game/XIRemix/Core/Player/Input/IMC_Exploration.IMC_Exploration" 0)
  (message `EnhancedInputSubsystemInterface.AddMappingContext` _returnvalue "/Game/XIRemix/Core/Player/Input/IMC_Target.IMC_Target" 0)
  (set `self.PlayerPawn` (`self.K2_GetPawn`)))

(event `EnhancedInput|/Game/XIRemix/Core/Player/Input/IA_Movement`
  (params (ActionValue :type "Vector2D Structure") (ElapsedSeconds :type "Float (single-precision)") (TriggeredSeconds :type "Float (single-precision)"))
  (bind (_x _y) (`KismetMathLibrary.BreakVector2D` ActionValue))
  (:`Triggered`
    (bind _playerpawn (`self.PlayerPawn`)
      (:`then`
        (bind _returnvalue (`Pawn.GetControlRotation` _playerpawn))
        (`Pawn.AddMovementInput` _playerpawn (`KismetMathLibrary.GetForwardVector` _returnvalue) _y false)
        (`Pawn.AddMovementInput` _playerpawn (`KismetMathLibrary.GetRightVector` _returnvalue) _x false))
      (:`else`))))

(event `EnhancedInput|/Game/XIRemix/Core/Player/Input/IA_CameraMovement`
  (params (ActionValue :type "Vector2D Structure") (ElapsedSeconds :type "Float (single-precision)") (TriggeredSeconds :type "Float (single-precision)"))
  (bind (_x _y) (`KismetMathLibrary.BreakVector2D` ActionValue))
  (:`Triggered`
    (bind _playerpawn (`self.PlayerPawn`)
      (:`then`
        (`Pawn.AddControllerPitchInput` _playerpawn _y)
        (`Pawn.AddControllerYawInput` _playerpawn _x))
      (:`else`))))

(fn `UserConstructionScript`)