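; Gameplay player controller that turns Enhanced Input into pawn movement, camera look and hostile target selection.
; On BeginPlay it adds movement and camera mappings, then retries every second until the pawn is valid to bind its XITargetSystemComponent and add target mappings.
; Movement follows control yaw and is gated by CanMove.
; Target events create or remove the target plate widget and set or clear the pawn's main target.
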(event `self.ReceiveBeginPlay`
  (bind _returnvalue (pcsubsystem `EnhancedInputLocalPlayerSubsystem` self))
  (message `EnhancedInputSubsystemInterface.AddMappingContext` _returnvalue "/Game/XIRemix/Core/Player/Input/IMC_Movement.IMC_Movement" 0)
  (message `EnhancedInputSubsystemInterface.AddMappingContext` _returnvalue "/Game/XIRemix/Core/Player/Input/IMC_CameraControl.IMC_CameraControl" 0)
  (bind _playerpawn (`self.PlayerPawn` :!label _label)
    (:`then`
      (bind _output_get (set `self.XITargetSystemComponent` (`CombatFunctionLibrary.GetXITargetSystemComponent` _playerpawn)))
      (add `XITargetSystemComponent.OnTargetSelected` _output_get (`|CreateDelegate` :!event `TargetSelected`))
      (add `XITargetSystemComponent.OnTargetRemoved` _output_get (`|CreateDelegate` :!event `TargetRemoved`))
      (message `EnhancedInputSubsystemInterface.AddMappingContext` _returnvalue "/Game/XIRemix/Core/Player/Input/IMC_Target.IMC_Target" 0))
    (:`else`
      (`KismetSystemLibrary.Delay` 1.0)
      (goto _label))))

(event `EnhancedInput|/Game/XIRemix/Core/Player/Input/IA_Movement`
  (params (ActionValue :type "Vector2D Structure") (ElapsedSeconds :type "Float (single-precision)") (TriggeredSeconds :type "Float (single-precision)"))
  (bind (_x _y) (`KismetMathLibrary.BreakVector2D` ActionValue))
  ;[1 1 1] Movement + Camera
  (:`Triggered`
    (bind _playerpawn (`self.PlayerPawn`)
      (:`then`
        (if (`self.bCanMove`)
          (bind (_returnvalue_roll _returnvalue_pitch _returnvalue_yaw) (`KismetMathLibrary.BreakRotator` (`Pawn.GetControlRotation` _playerpawn)))
          (`Pawn.AddMovementInput` _playerpawn (`KismetMathLibrary.GetForwardVector` (`KismetMathLibrary.MakeRotator` 0.0 0.0 _returnvalue_yaw)) _y false)
          (`Pawn.AddMovementInput` _playerpawn (`KismetMathLibrary.GetRightVector` (`KismetMathLibrary.MakeRotator` 0.0 0.0 _returnvalue_yaw)) _x false)))
      (:`else`))))

(event `XIGameplayControllerInterface.SetIsMoveable`
  (params (bIsMoveable :type Boolean))
  ;[1 1 1] Movement + Camera
  (set `self.bCanMove` bIsMoveable))

(event `EnhancedInput|/Game/XIRemix/Core/Player/Input/IA_CameraMovement`
  (params (ActionValue :type "Vector2D Structure") (ElapsedSeconds :type "Float (single-precision)") (TriggeredSeconds :type "Float (single-precision)"))
  (bind (_x _y) (`KismetMathLibrary.BreakVector2D` ActionValue))
  ;[1 1 1] Movement + Camera
  (:`Triggered`
    (bind _playerpawn (`self.PlayerPawn`)
      (:`then`
        (`Pawn.AddControllerPitchInput` _playerpawn _y)
        (`Pawn.AddControllerYawInput` _playerpawn _x))
      (:`else`))))

(event `EnhancedInput|/Game/XIRemix/Core/Player/Input/IA_TargetRight`
  (params (ActionValue :type "Float (single-precision)") (ElapsedSeconds :type "Float (single-precision)") (TriggeredSeconds :type "Float (single-precision)"))
  ;[1 1 1] Target System + UI
  (:`Triggered`
    (`XITargetSystemComponent.TargetActor` (`self.XITargetSystemComponent`) "Hostile" ActionValue)))

(event `EnhancedInput|/Game/XIRemix/Core/Player/Input/IA_TargetLock`
  (params (ActionValue :type Boolean) (ElapsedSeconds :type "Float (single-precision)") (TriggeredSeconds :type "Float (single-precision)"))
  ;[1 1 1] Target System + UI
  (:`Triggered`
    (`XITargetSystemComponent.LockCamera` (`self.XITargetSystemComponent`))))

(event `TargetSelected`
  (params (TargetActor :type "Actor Object Reference"))
  ;[1 1 1] Target System + UI
  (`self.TargetUI`
    (:`then`)
    (:`else`
      (bind _returnvalue (`|CreateWidget` "/Game/XIRemix/Core/Player/UI/WBP_TargetPlate.WBP_TargetPlate_C" self TargetActor))
      (bind _output_get (set `self.TargetUI` _returnvalue))
      (`UserWidget.AddToViewport` _output_get 0)
      (`CombatFunctionLibrary.SetMainTarget` (`self.PlayerPawn`) TargetActor))))

(event `TargetRemoved`
  (params (TargetActor :type "Actor Object Reference"))
  ;[1 1 1] Target System + UI
  (bind _targetui (`self.TargetUI`)
    (:`then`
      (`Widget.RemoveFromParent` _targetui)
      (set `self.TargetUI` null)
      (`CombatFunctionLibrary.SetMainTarget` (`self.PlayerPawn`)))
    (:`else`)))

(fn `UserConstructionScript`)